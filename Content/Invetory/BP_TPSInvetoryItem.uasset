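; BP_TPSInvetoryItem is an inventory item actor whose look is built from its InvetoryData.
; The Construction Script picks a sphere, cube or cylinder mesh from the item type and shows the score on a text render.
; It also creates a dynamic instance of M_BaseColor and sets its Color to a random ColorPallete entry.
; The event graph holds only disabled placeholder events, so this Blueprint adds no runtime logic.
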(event EventBeginPlay)

(event Collision|EventActorBeginOverlap
  (params (OtherActor :type Actor%20Object%20Reference)))

(event EventTick
  (params (DeltaSeconds :type Float%20%28single-precision%29)))

(fn ConstructionScript
  (bind _invetorydata (Variables|Default|GetInvetoryData))
  (Components|StaticMesh|SetStaticMesh (Variables|Default|GetMaterialSphere) (Utilities|Select :Index (.type _invetorydata) :SPHERE "/Engine/BasicShapes/Sphere.Sphere" :CUBE "/Game/Geometry/Meshes/1M_Cube.1M_Cube" :CYLIDER "/Engine/BasicShapes/Cylinder.Cylinder"))
  (Rendering|Components|TextRender|SetText (Variables|Default|GetTextRender) (Utilities|Text|ToText(Integer) (.score _invetorydata)))
  (bind _returnvalue (Rendering|Material|CreateDynamicMaterialInstance (Variables|Default|GetMaterialSphere) 0 "/Game/Invetory/M_BaseColor.M_BaseColor" "None" :!class /Script/Engine.PrimitiveComponent))
  (Rendering|Material|SetVectorParameterValue _returnvalue "Color" (.OutItem (Utilities|Array|Random (Variables|Default|GetColorPallete))) :!class /Script/Engine.MaterialInstanceDynamic))