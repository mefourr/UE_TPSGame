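; BP_Test_TPSInvetoryItem is a test inventory item actor that displays its type and score as a colored mesh and text.
; The construction script selects a shape from InvetoryData, shows the score, and applies a random palette color to a dynamic material and the text.
; SetInventoryData stores data and color, then calls Init; GenerateColor returns that stored color.
; An explosion emitter spawns at the actor's location on EndPlay.
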(event Custom|SetTestData)

(event Custom|SetInventoryData
  (params (InvData :type Invetory%20Data%20Structure) (Color :type Linear%20Color%20Structure))
  (Variables|Default|SetInvetoryData InvData)
  (Variables|Default|SetTestColor Color)
  (CallFunction|Init))

(event Collision|EventActorBeginOverlap
  (params (OtherActor :type Actor%20Object%20Reference)))

(event EventTick
  (params (DeltaSeconds :type Float%20%28single-precision%29)))

(event EventEndPlay
  (params (EndPlayReason :type EEndPlayReason%20Enum :default "Destroyed"))
  (Effects|SpawnEmitteratLocation "/Game/StarterContent/Particles/P_Explosion.P_Explosion" (Transformation|GetActorLocation)))

(event EventBeginPlay)

(fn ConstructionScript
  (bind _invetorydata (Variables|Default|GetInvetoryData))
  (Components|StaticMesh|SetStaticMesh (Variables|Default|GetStaticMesh) (Utilities|Select :Index (.type _invetorydata) :SPHERE "/Engine/BasicShapes/Sphere.Sphere" :CUBE "/Game/Geometry/Meshes/1M_Cube.1M_Cube" :CYLIDER "/Engine/BasicShapes/Cylinder.Cylinder" :CONE "/Engine/BasicShapes/Cone.Cone"))
  (Rendering|Components|TextRender|SetText (Variables|Default|GetTextRender_0) (Utilities|Text|ToText(Integer) (.score _invetorydata)))
  (bind _returnvalue (Rendering|Material|CreateDynamicMaterialInstance (Variables|Default|GetStaticMesh) 0 "/Game/Invetory/M_BaseColor.M_BaseColor" "None" :!class /Script/Engine.PrimitiveComponent))
  (bind _output_get (LocalVariables|SetColorToSet (.OutItem (Utilities|Array|Random (Variables|Default|GetColorPallete_0)))))
  (Rendering|Material|SetVectorParameterValue _returnvalue "Color" _output_get :!class /Script/Engine.MaterialInstanceDynamic)
  (Rendering|Components|TextRender|SetTextRenderColor (Variables|Default|GetTextRender_0) (Math|Conversions|ToColor(LinearColor) (LocalVariables|GetColorToSet))))

(fn GenerateColor
  (return (Variables|Default|GetTestColor)))