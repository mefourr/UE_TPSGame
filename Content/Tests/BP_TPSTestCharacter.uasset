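; BP_TPSTestCharacter is a test character Blueprint that displays its current health as text.
; Every tick it converts GetHealthPercent to a whole number out of 100 and writes it to a TextRender component.
; A SetHealthData event stores the incoming HealthData in the matching variable, while BeginPlay only calls the parent.
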(event Custom|SetHealthData
  (params (HealthData :type Health%20Data%20Structure))
  (Variables|Default|SetHealthData HealthData))

(event EventBeginPlay
  (|CallParentFunction))

(event Collision|EventActorBeginOverlap
  (params (OtherActor :type Actor%20Object%20Reference))
  (|CallParentFunction OtherActor) ; This node is disabled and will not be called.\nDrag off pins to build functionality.
)

(event EventTick
  (params (DeltaSeconds :type Float%20%28single-precision%29))
  (|CallParentFunction DeltaSeconds)
  (Rendering|Components|TextRender|SetText (Variables|Default|GetTextRender) (Utilities|Text|ToText(String) (Class|KismetMathLibrary|ToInt64(Float) (* (Class|TPSCharacter|GetHealthPercent) 1e+02)))))

(fn ConstructionScript
  (|CallParentFunction))